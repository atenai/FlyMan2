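; Game mode for FlyMan2 that holds a player respawn event and shows or hides a test text widget.
; Custom events, named as calls from the player, add and remove the widget, since comments note the game mode gets no key input.
; RespawnPlayer spawns a character at a player start, possesses it and rebinds to its destruction.
; The initial respawn binding and score widget creation are disconnected, and BeginPlay is empty.
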(event `Key|Two`
  (params (Key :type "Key Structure"))
  ;[1 1 1] ゲームモードはキー入力に対応していない
  (:`Pressed`
    (`KismetSystemLibrary.PrintString` "2_True"))
  (:`Released`
    (`KismetSystemLibrary.PrintString` "2_False")))

(event `self.ReceiveBeginPlay`
  ;[1 1 1] プレイヤーのリスポーンシステム4.7.6でしか使用できない
)

(event `RespawnPlayer` :!signature `self.OnDestroyed`
  (params (DestroyedActor :type "Actor Object Reference"))
  ;[1 1 1] プレイヤーのリスポーンシステム4.7.6でしか使用できない
  (bind _returnvalue (`|SpawnActorFromClass` "/Game/FlyMan2/Character/FlyMan2_Character.FlyMan2_Character_C" (`self.GetTransform` (`self.K2_FindPlayerStart` null)) "AdjustIfPossibleButDontSpawnIfColliding" "OverrideRootScale" null null))
  (`Controller.Possess` (`GameplayStatics.GetPlayerController` 0) _returnvalue)
  (add `self.OnDestroyed` _returnvalue (delegate `RespawnPlayer`)))

(event `UITrue_Player->GameMode`
  ;[1 1 1] UIを表示する、しかしゲームモードはキー入力に対応していない為、カスタムイベントで対応しなくてはいけない
  (bind _returnvalue (`|CreateWidget` "/Game/FlyMan2/UMG/IntroductionToBlueprints/UI01_TestText.UI01_TestText_C"))
  (set `self.UI_FlyMan2_GameMode` _returnvalue)
  (`UserWidget.AddToViewport` _returnvalue 0))

(event `UIFalse_Player->GameMode`
  ;[1 1 1] UIを非表示
  (`Widget.RemoveFromParent` (`self.UI_FlyMan2_GameMode`)))

(fn `UserConstructionScript`)
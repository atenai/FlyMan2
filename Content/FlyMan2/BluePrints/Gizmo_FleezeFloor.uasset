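; An ice-floor gizmo that makes the player character slide while inside its box collision.
; Overlap begin zeroes the character's ground friction and walking braking and adds it to a slipping list; overlap end writes back fixed values and removes it.
; Each Tick cuts acceleration for listed characters at or above a speed threshold, locking out steering until they slow down, when acceleration returns.
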(event `self.ReceiveBeginPlay`)

(event `self.ReceiveActorBeginOverlap`
  (params (OtherActor :type "Actor Object Reference")))

(event `self.ReceiveTick`
  (params (DeltaSeconds :type "Float (single-precision)"))
  (for _array_element (`self.SlippingCharacterList`)
    (if (< (`KismetMathLibrary.VSize` (`self.GetVelocity` _array_element)) 200.0)
      (bind _charactermovement (`Character.CharacterMovement` _array_element))
      (set `CharacterMovementComponent.MaxAcceleration` 2048.0 _charactermovement)
      (else
        (set `CharacterMovementComponent.MaxAcceleration` 0.0 _charactermovement)))))

(event `self.Box.OnComponentBeginOverlap`
  (params (OtherActor :type "Actor Object Reference") (OtherComp :type "PrimitiveComponent Object Reference") (OtherBodyIndex :type Integer) (bFromSweep :type Boolean) (SweepResult :type "EngineTypes.HitResult Structure (by ref)"))
  (if (== OtherActor (`GameplayStatics.GetPlayerPawn` 0))
    (bind _ascharacter (cast `Character` OtherActor))
    (bind _charactermovement (`Character.CharacterMovement` _ascharacter))
    (set `CharacterMovementComponent.GroundFriction` 0.0 _charactermovement) ; 地上での摩擦係数の設定
    (set `CharacterMovementComponent.BrakingDecelerationWalking` 0.0 _charactermovement) ; 歩行時のブレーキ能力の設定
    (`KismetArrayLibrary.Array_Add` (`self.SlippingCharacterList`) _ascharacter)))

(event `self.Box.OnComponentEndOverlap`
  (params (OtherActor :type "Actor Object Reference") (OtherComp :type "PrimitiveComponent Object Reference") (OtherBodyIndex :type Integer))
  (if (== OtherActor (`GameplayStatics.GetPlayerPawn` 0))
    (bind _ascharacter (cast `Character` OtherActor))
    (bind _charactermovement (`Character.CharacterMovement` _ascharacter))
    (set `CharacterMovementComponent.GroundFriction` 3.0 _charactermovement) ; 地上での摩擦係数の設定
    (set `CharacterMovementComponent.BrakingDecelerationWalking` 2048.0 _charactermovement) ; 歩行時のブレーキ能力の設定
    (`KismetArrayLibrary.Array_RemoveItem` (`self.SlippingCharacterList`) _ascharacter)
    (set `CharacterMovementComponent.MaxAcceleration` 2048.0 _charactermovement)))

(fn `UserConstructionScript`)
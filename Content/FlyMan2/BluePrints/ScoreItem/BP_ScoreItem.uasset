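; BP_ScoreItem is a score pickup in FlyMan2 that the player collects by touching it.
; When the player pawn enters its sphere collision, it adds one point to the score on FlyMan2_PlayerController, prints the total, spawns an explosion effect and destroys itself.
; Disconnected variants store the score on the character or game mode instead, with a note that character-held score is lost when the character is destroyed.
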(event `self.ReceiveBeginPlay`)

(event `self.ReceiveActorBeginOverlap`
  (params (OtherActor :type "Actor Object Reference")))

(event `self.ReceiveTick`
  (params (DeltaSeconds :type "Float (single-precision)")))

(event `self.SphereCol.OnComponentBeginOverlap`
  (params (OtherActor :type "Actor Object Reference") (OtherComp :type "PrimitiveComponent Object Reference") (OtherBodyIndex :type Integer) (bFromSweep :type Boolean) (SweepResult :type "EngineTypes.HitResult Structure (by ref)"))
  (if (== OtherActor (`GameplayStatics.GetPlayerPawn` 0))
    ;[1 1 1] プレイヤーコントローラーに変数を持たせたバージョン
    (bind _asfly_man_2_player_controller (cast `/Game/FlyMan2/BluePrints/FlyMan2_PlayerController` (`GameplayStatics.GetPlayerController` 0)))
    (bind _output_get (set `/Game/FlyMan2/BluePrints/FlyMan2_PlayerController.Score_FlyMan2_PlayerController` (+ (`/Game/FlyMan2/BluePrints/FlyMan2_PlayerController.Score_FlyMan2_PlayerController` _asfly_man_2_player_controller) 1) _asfly_man_2_player_controller))
    (`KismetSystemLibrary.PrintString` (`KismetStringLibrary.Conv_IntToString` _output_get))
    (`GameplayStatics.SpawnEmitterAtLocation` "/Game/StarterContent/Particles/P_Explosion.P_Explosion" (`self.K2_GetActorLocation`))
    (`self.K2_DestroyActor`)))

(fn `UserConstructionScript`)
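; Electric gate gizmo that periodically switches on and knocks away characters touching it.
; A looping timer calls ActivateGate, which turns on the particle effect and a Damage flag briefly, then switches both off.
; While the flag is set, Tick polls actors overlapping the Box and launches Characters away from the gate's location, overriding their velocity.
; Despite the flag's name, no damage is applied.
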(event `self.ReceiveBeginPlay`
  (`KismetSystemLibrary.K2_SetTimer` null "ActivateGate" 4.0 true))

(event `self.ReceiveTick`
  (params (DeltaSeconds :type "Float (single-precision)"))
  (if (`self.bDamage`)
    (for _array_element (`PrimitiveComponent.GetOverlappingActors` (`self.Box`) null)
      (bind _ascharacter (cast `Character` _array_element))
      (`Character.LaunchCharacter` _ascharacter (* (`KismetMathLibrary.GetForwardVector` (`KismetMathLibrary.FindLookAtRotation` (`self.K2_GetActorLocation`) (`self.K2_GetActorLocation` _ascharacter))) 1000.0) true true))))

(event `ActivateGate`
  (set `self.bDamage` true)
  (`ActorComponent.SetActive` (`self.ParticleSystem`) true false)
  (`KismetSystemLibrary.Delay` 1.0)
  (set `self.bDamage` false)
  (`ActorComponent.SetActive` (`self.ParticleSystem`) false false))

(fn `UserConstructionScript`)
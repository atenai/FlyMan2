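; FlyMan2's player controller Blueprint handles pausing and quitting the game.
; The P key toggles game pause, creating and showing a new pause widget when pausing and removing it from the viewport when resuming.
; The Quit input action, noted as the Q key for builds, exits the game.
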(event `Key|P` :consume false :paused true :overrideparent false
  (params (Key :type "Key Structure"))
  (:`Pressed`
    ;[1 1 1] ポーズシステム
    (if (`GameplayStatics.IsGamePaused`)
      (`GameplayStatics.SetGamePaused` false)
      ;;[1 1 1] UIを非表示にする
      (`Widget.RemoveFromParent` (`self.PauseWidget`))
      (else
        (`GameplayStatics.SetGamePaused` true)
        ;;[1 1 1] UIを表示する
        (bind _returnvalue (`|CreateWidget` "/Game/FlyMan2/UMG/Widget_Pause.Widget_Pause_C"))
        (bind _output_get (set `self.PauseWidget` _returnvalue))
        (`UserWidget.AddToViewport` _output_get 0)))))

(event `InputAction|Quit`
  (params (Key :type "Key Structure"))
  (:`Pressed`
    (`KismetSystemLibrary.QuitGame` null "Quit") ; ビルドでのゲームプレイの際にQキーでゲームを終了する
  ))

(fn `UserConstructionScript`)
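; Gizmo_BlinkStep is a blinking step gizmo whose static mesh alternately appears and disappears on a timer.
; Tick counts BlinkCount down by delta time, then flips the Appear state and reloads the count from AppearRate or DisAppearRate.
; Each flip toggles mesh visibility and collision together.
; On reappearing it also spawns a spark emitter and plays an explosion sound at the actor's location.
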(event `self.ReceiveBeginPlay`)

(event `self.ReceiveActorBeginOverlap`
  (params (OtherActor :type "Actor Object Reference")))

(event `self.ReceiveTick`
  (params (DeltaSeconds :type "Float (single-precision)"))
  (bind _returnvalue (`self.K2_GetActorLocation`))
  (bind _staticmesh (`self.StaticMesh`))
  (bind _staticmesh_2 (`self.StaticMesh`))
  (set `self.DeltaTime` DeltaSeconds) ; 毎フレームである0.04をセット
  (if (`self.bAppear`)
    (bind _output_get (set `self.BlinkCount` (- (`self.BlinkCount`) (`self.DeltaTime`))))
    (if (<= _output_get 0.0)
      (`SceneComponent.SetVisibility` _staticmesh_2 false false) ; 表示を消す（チェックマークなし）
      (`PrimitiveComponent.SetCollisionEnabled` _staticmesh_2 "NoCollision") ; コリジョンを消す
      (set `self.bAppear` false)
      (set `self.BlinkCount` (`self.DisAppearRate`)))
    (else
      (bind _output_get_2 (set `self.BlinkCount` (- (`self.BlinkCount`) (`self.DeltaTime`))))
      (if (<= _output_get_2 0.0)
        (`SceneComponent.SetVisibility` _staticmesh true false) ; 表示する（チェックマークあり）
        (`PrimitiveComponent.SetCollisionEnabled` _staticmesh "QueryAndPhysics") ; コリジョンを出す
        (set `self.bAppear` true)
        (set `self.BlinkCount` (`self.AppearRate`))
        (`GameplayStatics.SpawnEmitterAtLocation` "/Game/StarterContent/Particles/P_Sparks.P_Sparks" _returnvalue) ; エフェクトを表示する
        (`GameplayStatics.PlaySoundAtLocation` "/Game/StarterContent/Audio/Explosion_Cue.Explosion_Cue" _returnvalue) ; サウンドを鳴らす
      ))))

(fn `UserConstructionScript`)
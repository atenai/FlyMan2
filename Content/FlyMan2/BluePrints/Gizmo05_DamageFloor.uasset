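; Damage floor gimmick that hurts the player pawn and knocks it away on contact.
; When the player pawn begins overlapping the Box component, it takes fixed damage and a Japanese debug message announces the hit.
; If that pawn is a Character, it is launched along the look-at direction from the floor's origin to the pawn, added to its current velocity.
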(event `self.ReceiveBeginPlay`)

(event `self.ReceiveActorBeginOverlap`
  (params (OtherActor :type "Actor Object Reference")))

(event `self.ReceiveTick`
  (params (DeltaSeconds :type "Float (single-precision)")))

(event `self.Box.OnComponentBeginOverlap`
  (params (OtherActor :type "Actor Object Reference") (OtherComp :type "PrimitiveComponent Object Reference") (OtherBodyIndex :type Integer) (bFromSweep :type Boolean) (SweepResult :type "EngineTypes.HitResult Structure (by ref)"))
  (if (== OtherActor (`GameplayStatics.GetPlayerPawn` 0))
    (`GameplayStatics.ApplyDamage` OtherActor 20.0 null self)
    (`KismetSystemLibrary.PrintString` "ダメージ床を踏んだ。20のダメージ！" true true (struct :`R` 1.0 :`G` 0.5 :`B` 0.05 :`A` 1.0))
    (bind _ascharacter (cast `Character` OtherActor))
    (`Character.LaunchCharacter` _ascharacter (* (`KismetMathLibrary.GetForwardVector` (`KismetMathLibrary.FindLookAtRotation` (`self.K2_GetActorLocation`) (`self.K2_GetActorLocation` OtherActor))) 2000.0) false false)))

(fn `UserConstructionScript`)
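; Gizmo_Teleporter is a teleporter gizmo that moves the player pawn to the location of a referenced TeleportTarget.
; When the first player's pawn begins overlapping its Capsule and the target is valid, it sets the pawn's location without sweeping.
; It then spawns the P_Explosion particle effect at the destination.
; Only the pawn's location is set, and other overlapping actors are ignored.
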(event `self.ReceiveBeginPlay`)

(event `self.ReceiveActorBeginOverlap`
  (params (OtherActor :type "Actor Object Reference")))

(event `self.ReceiveTick`
  (params (DeltaSeconds :type "Float (single-precision)")))

(event `self.Capsule.OnComponentBeginOverlap`
  (params (OtherActor :type "Actor Object Reference") (OtherComp :type "PrimitiveComponent Object Reference") (OtherBodyIndex :type Integer) (bFromSweep :type Boolean) (SweepResult :type "EngineTypes.HitResult Structure (by ref)"))
  (if (== OtherActor (`GameplayStatics.GetPlayerPawn` 0))
    (if (`KismetSystemLibrary.IsValid` (`self.TeleportTarget`))
      (`self.K2_SetActorLocation` OtherActor (`self.K2_GetActorLocation` (`self.TeleportTarget`)) false)
      (`GameplayStatics.SpawnEmitterAtLocation` "/Game/StarterContent/Particles/P_Explosion.P_Explosion" (`self.K2_GetActorLocation` (`self.TeleportTarget`))))))

(fn `UserConstructionScript`)
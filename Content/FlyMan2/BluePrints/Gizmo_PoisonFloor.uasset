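; Poison floor gizmo that deals periodic damage to Characters standing inside its Box volume.
; Box overlap begin and end events add and remove Characters in DamagedCharacterList.
; A looping timer started on BeginPlay calls PoisonDamage every DamageRate seconds, applying Damage to each listed Character and printing a debug message.
; A spark emitter node is present but unconnected, so no effect plays.
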(event `self.ReceiveActorBeginOverlap`
  (params (OtherActor :type "Actor Object Reference")))

(event `self.ReceiveTick`
  (params (DeltaSeconds :type "Float (single-precision)")))

(event `self.ReceiveBeginPlay`
  ;[1 1 1] SetTimerのFunctionNameに書いたカスタムイベント（PoisonDamage）を呼び出す
  (`KismetSystemLibrary.K2_SetTimer` null "PoisonDamage" (`self.DamageRate`) true))

(event `PoisonDamage`
  ;[1 1 1] SetTimerのFunctionNameに書いたカスタムイベント（PoisonDamage）を呼び出す
  (for _array_element (`self.DamagedCharacterList`)
    (`GameplayStatics.ApplyDamage` _array_element (`self.Damage`) null self)
    (`KismetSystemLibrary.PrintString` "毒により10ダメージ" true true (struct :`R` 0.6 :`B` 1.0 :`A` 1.0))))

(event `self.Box.OnComponentBeginOverlap`
  (params (OtherActor :type "Actor Object Reference") (OtherComp :type "PrimitiveComponent Object Reference") (OtherBodyIndex :type Integer) (bFromSweep :type Boolean) (SweepResult :type "EngineTypes.HitResult Structure (by ref)"))
  (bind _ascharacter (cast `Character` OtherActor))
  (`KismetArrayLibrary.Array_Add` (`self.DamagedCharacterList`) _ascharacter))

(event `self.Box.OnComponentEndOverlap`
  (params (OtherActor :type "Actor Object Reference") (OtherComp :type "PrimitiveComponent Object Reference") (OtherBodyIndex :type Integer))
  (bind _ascharacter (cast `Character` OtherActor))
  (`KismetArrayLibrary.Array_RemoveItem` (`self.DamagedCharacterList`) _ascharacter))

(fn `UserConstructionScript`)
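; Light actor for FlyMan2 whose component visibility follows the boolean BPointLightHensuu, applied every Tick.
; Its Box overlap only casts to FlyMan2_Character, and the custom events meant for the player and Map1 just print debug text, as do the 1-key handlers.
; Unconnected leftover nodes hold a timed light flash, game-clear widget show and hide, and a MapGameClear level load, so none of these run.
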(event `self.ReceiveTick`
  (params (DeltaSeconds :type "Float (single-precision)"))
  (`SceneComponent.SetVisibility` (`self.b_PointLight_Hensuu`)) ; アクターの可視化
)

(event `self.Box.OnComponentBeginOverlap`
  (params (OverlappedComponent :type "PrimitiveComponent Object Reference") (OtherActor :type "Actor Object Reference") (OtherComp :type "PrimitiveComponent Object Reference") (OtherBodyIndex :type Integer) (bFromSweep :type Boolean) (SweepResult :type "HitResult Structure (by ref)"))
  ;[1 1 1] ライトからプレイヤーのカスタムイベントにアクセス
  (cast `/Game/FlyMan2/Character/FlyMan2_Character` OtherActor))

(event `Player->Light`
  ;[1 1 1] プレイヤーからライトのカスタムイベントの呼び出し
  (`KismetSystemLibrary.PrintString` "Player->Light"))

(event `Map1->Light`
  ;[1 1 1] マップ１からライトのカスタムイベントの呼び出し
  (`KismetSystemLibrary.PrintString` "Map1->Light"))

(event `Key|One`
  (params (Key :type "Key Structure"))
  ;[1 1 1] アクターはキー入力に対応していない
  (:`Pressed`
    (`KismetSystemLibrary.PrintString` "1_True"))
  (:`Released`
    (`KismetSystemLibrary.PrintString` "1_False")))

(fn `UserConstructionScript`)
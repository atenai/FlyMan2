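; Falling floor actor that drops when the player steps on it and respawns at its original transform.
; BeginPlay saves the transform, and a one-shot box overlap with a "Player"-tagged actor sets a flag, then after short delays enables mesh physics and destroys the actor.
; Tick polls that flag and, after its own delay, spawns a fresh copy at the saved transform shortly before the old one is destroyed.
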(event `self.ReceiveTick`
  (params (DeltaSeconds :type "Float (single-precision)"))
  (if (`self.b_FallFloorCol`)
    ;[1 1 1] アクターをリスポーンする
    (`KismetSystemLibrary.Delay` 2.5)
    (`|SpawnActorFromClass` "FallFloor_Actor_Blueprint_C" (`self.FallFloorPos`) "AlwaysSpawn" "OverrideRootScale" null null)
    (set `self.b_FallFloorCol` false) ; b_FallFloorColをFalseにする
    (`KismetSystemLibrary.PrintString` "RespawnFallFloor")))

(event `self.ReceiveBeginPlay`
  ;[1 1 1] リスポーンする座標を最初に取得する
  (set `self.FallFloorPos` (`self.GetTransform`)) ; 座標を入れておく
  (`KismetSystemLibrary.PrintString` "SetFallFloorPos"))

(event `self.BoxCol.OnComponentBeginOverlap`
  (params (OverlappedComponent :type "PrimitiveComponent Object Reference") (OtherActor :type "Actor Object Reference") (OtherComp :type "PrimitiveComponent Object Reference") (OtherBodyIndex :type Integer) (bFromSweep :type Boolean) (SweepResult :type "HitResult Structure (by ref)"))
  ;[1 1 1] タグによるPlayerキャラクターの判別
  (if (`self.ActorHasTag` OtherActor "Player")
    (`/Engine/EditorBlueprintResources/StandardMacros.DoOnce` false ; １度だけ実行する
      (:`Completed`
        (set `self.b_FallFloorCol` true) ; b_FallFloorColをTrueにする
        (`KismetSystemLibrary.PrintString` "FallFloor_Player_Atari")
        ;[1 1 1] 床の物理がオンになり床が落ちていく
        (`KismetSystemLibrary.Delay` 1.0) ; １秒間待つ
        (`PrimitiveComponent.SetSimulatePhysics` (`self.StaticMeshComponent`) true) ; 物理シミュレーションをオンにする
        (`KismetSystemLibrary.Delay` 2.0) ; ２秒待つ
        (`self.K2_DestroyActor`) ; このアクターを消す
      ))))

(fn `UserConstructionScript`)